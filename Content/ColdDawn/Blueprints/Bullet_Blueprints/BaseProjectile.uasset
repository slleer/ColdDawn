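; Base projectile Blueprint for bullets that deal damage to what they hit and then disappear.
; On Hit, it applies BulletDamage only if the other actor's root component has the tag "None", and destroys itself either way.
; SetDamage lets the damage value be set from outside and prints it as debug output.
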(event `self.ReceiveHit`
  (params (MyComp :type "PrimitiveComponent Object Reference") (Other :type "Actor Object Reference") (OtherComp :type "PrimitiveComponent Object Reference") (bSelfMoved :type Boolean) (HitLocation :type "Vector Structure") (HitNormal :type "Vector Structure") (NormalImpulse :type "Vector Structure") (Hit :type "HitResult Structure (by ref)"))
  ;[1 1 1] Causes the bullet to dissapear when it doesn't hit an enemy and cause damage if does
  (if (`ActorComponent.ComponentHasTag` (`Actor.RootComponent` Other) "None")
    (`GameplayStatics.ApplyDamage` Other (`self.BulletDamage`))
    (`self.K2_DestroyActor`)
    (else
      (`self.K2_DestroyActor`))))

(fn `SetDamage`
  (params (InsertedDamage :type "Float (double-precision)"))
  (bind _output_get (set `self.BulletDamage` InsertedDamage))
  (`KismetSystemLibrary.PrintString` (`KismetStringLibrary.Conv_DoubleToString` _output_get)))

(fn `UserConstructionScript`)